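; AI enemy pawn that, depending on TypeOfRotation, either watches for the player or turns to a random yaw every second.
; In watch mode it smoothly faces an uncamouflaged player within 5 m and marks them dead after a short delay.
; Detection and rotation run as self-calling Delay loops, re-acquiring the player after their death.
; Tick handles the pawn's own death animation and destruction.
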(event `self.ReceiveBeginPlay`
  ;[1 1 1] Start Get Player
  (bind _astop_down_character (cast `/Game/TopDownBP/Blueprints/TopDownCharacter` (`GameplayStatics.GetPlayerCharacter` 0))) ; Get BP of Player
  (set `self.ActorPreview` _astop_down_character) ; Stock BP of Player
  (if (`self.TypeOfRotation`)
    (`self.Detect Event`) ; Launch Detection of player
    (else
      (`self.Random Rotation`))))

(event `FaceToPlayer`
  (bind (_returnvalue_roll _returnvalue_pitch _returnvalue_yaw) (`KismetMathLibrary.BreakRotator` (`KismetMathLibrary.RInterpTo` (`self.K2_GetActorRotation`) (`KismetMathLibrary.FindLookAtRotation` (`self.K2_GetActorLocation`) (`self.K2_GetActorLocation` (`self.ActorPreview`))) (`GameplayStatics.GetWorldDeltaSeconds`) 5.0)))
  ;[1 1 1] Look At System
  ;;[1 1 1] Always Face to Player
  (if (not (`self.IsDead`))
    (if (not (`/Game/TopDownBP/Blueprints/TopDownCharacter.IsDead` (`self.ActorPreview`)))
      (if (`self.CanRotate`)
        (`self.K2_SetActorRotation` (`KismetMathLibrary.MakeRotator` 0.0 0.0 _returnvalue_yaw)) ; Update Rotation
        (`KismetSystemLibrary.Delay` 0.001)
        (`self.FaceToPlayer`)
        (else
          (`self.Detect Event`)))
      (else
        (`self.GetPlayer`)))))

(event `Random Rotation`
  (bind (_returnvalue_roll _returnvalue_pitch _returnvalue_yaw) (`KismetMathLibrary.BreakRotator` (`KismetMathLibrary.RInterpTo` (`self.K2_GetActorRotation`) (`self.GetRotation`) (`GameplayStatics.GetWorldDeltaSeconds`) 200.0)))
  ;[1 1 1] Random Rotation
  (if (not (`self.IsDead`))
    (set `self.GetRotation` (`KismetMathLibrary.RandomRotator` true))
    (`self.K2_SetActorRotation` (`KismetMathLibrary.MakeRotator` 0.0 0.0 _returnvalue_yaw)) ; Update Rotation
    (`KismetSystemLibrary.PrintString` (`KismetStringLibrary.Conv_DoubleToString` _returnvalue_yaw))
    (`KismetSystemLibrary.Delay` 1.0)
    (`self.Random Rotation`)))

(event `Detect Event`
  (bind _actorpreview (`self.ActorPreview`))
  ;[1 1 1] Look At System
  ;;[1 1 1] Check is player is around of AI
  (if (not (`self.IsDead`))
    (if (not (`/Game/TopDownBP/Blueprints/TopDownCharacter.IsDead` (`self.ActorPreview`)))
      (if (not (`/Game/TopDownBP/Blueprints/TopDownCharacter.IsCamouflage` _actorpreview))
        (if (<= (`self.GetDistanceTo` _actorpreview) 500.0)
          (set `self.CanRotate` true) ; Enable Rotation
          (`self.FaceToPlayer`)
          (`KismetSystemLibrary.Delay` 0.5)
          (set `/Game/TopDownBP/Blueprints/TopDownCharacter.IsDead` true (`self.ActorPreview`))
          (else
            (set `self.CanRotate` false :!label _label)))
        (else
          (goto _label)))
      (`KismetSystemLibrary.Delay` 0.001)
      (`self.Detect Event`)
      (else
        (`self.GetPlayer`)))))

(event `self.ReceiveTick`
  (params (DeltaSeconds :type "Float (single-precision)"))
  ;[1 1 1] Destroy Actor
  (if (`self.IsDead`)
    (if (not (`self.PredictionDead`))
      (set `self.PredictionDead` true)
      (`SkeletalMeshComponent.PlayAnimation` (`self.Mesh`) "/Game/Assets/Animation/FallingForwardDeath_UE.FallingForwardDeath_UE" false)
      (`KismetSystemLibrary.Delay` 2.0)
      (`self.K2_DestroyActor`))))

(event `GetPlayer`
  ;[1 1 1] Look At System
  ;;[1 1 1] Get Player If Dead
  (`KismetSystemLibrary.Delay` 6.0)
  (bind _astop_down_character (cast `/Game/TopDownBP/Blueprints/TopDownCharacter` (`GameplayStatics.GetPlayerCharacter` 0))) ; Get BP of Player
  (set `self.ActorPreview` _astop_down_character) ; Stock BP of Player
  (`self.Detect Event`) ; Launch Detection of player
)

(fn `UserConstructionScript`)