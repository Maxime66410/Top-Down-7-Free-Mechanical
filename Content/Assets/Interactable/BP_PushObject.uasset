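; BP_PushObject is an interactable cube that the top-down player character can push.
; Overlap begin and end events on separate X and Y axis collision triggers call PushFunction to enable or disable pushing.
; PushFunction acts only on a TopDownCharacter that is not holding something, toggling the cube's physics simulation and the character's IsPush flag together.
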(event `self.Y Axis Collision.OnComponentBeginOverlap`
  (params (OverlappedComponent :type "PrimitiveComponent Object Reference") (OtherActor :type "Actor Object Reference") (OtherComp :type "PrimitiveComponent Object Reference") (OtherBodyIndex :type Integer) (bFromSweep :type Boolean) (SweepResult :type "HitResult Structure (by ref)"))
  (`self.PushFunction` OtherActor true) ; Call PUSH FUNCTION
)

(event `self.X Axis Collision.OnComponentBeginOverlap`
  (params (OverlappedComponent :type "PrimitiveComponent Object Reference") (OtherActor :type "Actor Object Reference") (OtherComp :type "PrimitiveComponent Object Reference") (OtherBodyIndex :type Integer) (bFromSweep :type Boolean) (SweepResult :type "HitResult Structure (by ref)"))
  (`self.PushFunction` OtherActor true) ; Call PUSH FUNCTION
)

(event `self.Y Axis Collision.OnComponentEndOverlap`
  (params (OverlappedComponent :type "PrimitiveComponent Object Reference") (OtherActor :type "Actor Object Reference") (OtherComp :type "PrimitiveComponent Object Reference") (OtherBodyIndex :type Integer))
  (`self.PushFunction` OtherActor) ; Call PUSH FUNCTION
)

(event `self.X Axis Collision.OnComponentEndOverlap`
  (params (OverlappedComponent :type "PrimitiveComponent Object Reference") (OtherActor :type "Actor Object Reference") (OtherComp :type "PrimitiveComponent Object Reference") (OtherBodyIndex :type Integer))
  (`self.PushFunction` OtherActor) ; Call PUSH FUNCTION
)

(fn `PushFunction`
  (params (Player :type "Actor Object Reference") (Physics :type Boolean))
  (bind _astop_down_character (cast `/Game/TopDownBP/Blueprints/TopDownCharacter` Player)) ; Detect if player
  (if (not (`/Game/TopDownBP/Blueprints/TopDownCharacter.IsHolding` _astop_down_character))
    (`PrimitiveComponent.SetSimulatePhysics` (`self.Cube`) Physics) ; Update Physique
    (set `/Game/TopDownBP/Blueprints/TopDownCharacter.IsPush` Physics _astop_down_character) ; Set Push
  ))

(fn `UserConstructionScript`)