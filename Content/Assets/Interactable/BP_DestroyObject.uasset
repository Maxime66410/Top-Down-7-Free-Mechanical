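; BP_DestroyObject is an interactable actor that removes itself from the world when the player character class is nearby and destruction is permitted.
; TargetCollision overlaps with a TopDownCharacter set CanDestroy on entry and clear it on exit.
; Tick polls PermissionDestroy and CanDestroy and destroys the actor when both are true.
; PermissionDestroy is only read here, never set.
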(event `self.ReceiveTick`
  (params (DeltaSeconds :type "Float (single-precision)"))
  (if (`self.PermissionDestroy`)
    (if (`self.CanDestroy`)
      (`self.K2_DestroyActor`))))

(event `self.TargetCollision.OnComponentBeginOverlap`
  (params (OverlappedComponent :type "PrimitiveComponent Object Reference") (OtherActor :type "Actor Object Reference") (OtherComp :type "PrimitiveComponent Object Reference") (OtherBodyIndex :type Integer) (bFromSweep :type Boolean) (SweepResult :type "HitResult Structure (by ref)"))
  (cast `/Game/TopDownBP/Blueprints/TopDownCharacter` OtherActor)
  (set `self.CanDestroy` true))

(event `self.TargetCollision.OnComponentEndOverlap`
  (params (OverlappedComponent :type "PrimitiveComponent Object Reference") (OtherActor :type "Actor Object Reference") (OtherComp :type "PrimitiveComponent Object Reference") (OtherBodyIndex :type Integer))
  (cast `/Game/TopDownBP/Blueprints/TopDownCharacter` OtherActor)
  (set `self.CanDestroy` false))

(fn `UserConstructionScript`)